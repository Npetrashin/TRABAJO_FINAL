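; Level 3 dialog component for "Evaluador", a Spanish-language examiner who quizzes the player with five arithmetic questions.
; Operations generates two-digit problems, limited to addition and subtraction because DivOrNot is always 1.
; The first correct answer is always listed first; later positions follow Condition variables, with random decoys.
; CorrectAmount, never reset here, gates the result: three or more opens MAP_2d_4, otherwise dialog index 1 offers a retry.
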(fn `Dialog`
  (locals (CorrectAmount :type Integer))
  (`parent.Dialog`)
  (switch `int` (`self.DialogTreeIndex`)
    (:`0`
      (bind (_state _optionindex) (`self.AddDialog` "Evaluador" "Perfecto, llegaste al final! Lista?" (`|MakeArray` "POR SUPUESTO!" "No..." :!type "Text")))
      (switch `/Game/assets/blueprints/enums/Enum_dialog` _state
        (:`NewEnumerator0`
          (switch `int` _optionindex
            (:`0`
              (bind (_question _result) (`self.Operations` :!label _label))
              (bind (_state_2 _optionindex_2) (`self.AddDialog` "Evaluador" (`KismetTextLibrary.Conv_StringToText` _question) (`|MakeArray` (`KismetTextLibrary.Conv_IntToText` _result) (`KismetTextLibrary.Conv_IntToText` (`KismetMathLibrary.RandomIntegerInRange` 1 99)) (`KismetTextLibrary.Conv_IntToText` (`KismetMathLibrary.RandomIntegerInRange` 1 99)))))
              (switch `/Game/assets/blueprints/enums/Enum_dialog` _state_2
                (:`NewEnumerator0`
                  (switch `int` _optionindex_2
                    (:`0`
                      (set `local.CorrectAmount` (+ (`local.CorrectAmount`) 1)))
                    (:`1`
                      _)
                    (:`2`
                      _))
                  (switch `int` (`self.condition`)
                    (:`0`
                      (bind (_question_2 _result_2) (`self.Operations`))
                      (bind (_state_3 _optionindex_3) (`self.AddDialog` "Evaluador" (`KismetTextLibrary.Conv_StringToText` _question_2) (`|MakeArray` (`KismetTextLibrary.Conv_IntToText` _result_2) (`KismetTextLibrary.Conv_IntToText` (`KismetMathLibrary.RandomIntegerInRange` 10 9999)) (`KismetTextLibrary.Conv_IntToText` (`KismetMathLibrary.RandomIntegerInRange` 10 9999)))))
                      (switch `/Game/assets/blueprints/enums/Enum_dialog` _state_3
                        (:`NewEnumerator0`
                          (switch `int` _optionindex_3
                            (:`0`
                              (set `local.CorrectAmount` (+ (`local.CorrectAmount`) 1)))
                            (:`1`
                              _)
                            (:`2`
                              _)))))
                    (:`1`
                      (bind (_question_3 _result_3) (`self.Operations`))
                      (bind (_state_4 _optionindex_4) (`self.AddDialog` "Evaluador" (`KismetTextLibrary.Conv_StringToText` _question_3) (`|MakeArray` (`KismetTextLibrary.Conv_IntToText` (`KismetMathLibrary.RandomIntegerInRange` 10 9999)) (`KismetTextLibrary.Conv_IntToText` _result_3) (`KismetTextLibrary.Conv_IntToText` (`KismetMathLibrary.RandomIntegerInRange` 10 9999)))))
                      (switch `/Game/assets/blueprints/enums/Enum_dialog` _state_4
                        (:`NewEnumerator0`
                          (switch `int` _optionindex_4
                            (:`0`
                              _)
                            (:`1`
                              (set `local.CorrectAmount` (+ (`local.CorrectAmount`) 1)))
                            (:`2`
                              _)))))
                    (:`2`
                      (bind (_question_4 _result_4) (`self.Operations`))
                      (bind (_state_5 _optionindex_5) (`self.AddDialog` "Evaluador" (`KismetTextLibrary.Conv_StringToText` _question_4) (`|MakeArray` (`KismetTextLibrary.Conv_IntToText` (`KismetMathLibrary.RandomIntegerInRange` 10 9999)) (`KismetTextLibrary.Conv_IntToText` (`KismetMathLibrary.RandomIntegerInRange` 10 9999)) (`KismetTextLibrary.Conv_IntToText` _result_4))))
                      (switch `/Game/assets/blueprints/enums/Enum_dialog` _state_5
                        (:`NewEnumerator0`
                          (switch `int` _optionindex_5
                            (:`0`
                              _)
                            (:`1`
                              _)
                            (:`2`
                              (set `local.CorrectAmount` (+ (`local.CorrectAmount`) 1))))))))
                  (switch `int` (`self.condition_0`)
                    (:`0`
                      (bind (_question_5 _result_5) (`self.Operations`))
                      (bind (_state_6 _optionindex_6) (`self.AddDialog` "Evaluador" (`KismetTextLibrary.Conv_StringToText` _question_5) (`|MakeArray` (`KismetTextLibrary.Conv_IntToText` _result_5) (`KismetTextLibrary.Conv_IntToText` (`KismetMathLibrary.RandomIntegerInRange` 10 9999)) (`KismetTextLibrary.Conv_IntToText` (`KismetMathLibrary.RandomIntegerInRange` 10 9999)))))
                      (switch `/Game/assets/blueprints/enums/Enum_dialog` _state_6
                        (:`NewEnumerator0`
                          (switch `int` _optionindex_6
                            (:`0`
                              (set `local.CorrectAmount` (+ (`local.CorrectAmount`) 1)))
                            (:`1`
                              _)
                            (:`2`
                              _)))))
                    (:`1`
                      (bind (_question_6 _result_6) (`self.Operations`))
                      (bind (_state_7 _optionindex_7) (`self.AddDialog` "Evaluador" (`KismetTextLibrary.Conv_StringToText` _question_6) (`|MakeArray` (`KismetTextLibrary.Conv_IntToText` (`KismetMathLibrary.RandomIntegerInRange` 10 9999)) (`KismetTextLibrary.Conv_IntToText` _result_6) (`KismetTextLibrary.Conv_IntToText` (`KismetMathLibrary.RandomIntegerInRange` 10 9999)))))
                      (switch `/Game/assets/blueprints/enums/Enum_dialog` _state_7
                        (:`NewEnumerator0`
                          (switch `int` _optionindex_7
                            (:`0`
                              _)
                            (:`1`
                              (set `local.CorrectAmount` (+ (`local.CorrectAmount`) 1)))
                            (:`2`
                              _)))))
                    (:`2`
                      (bind (_question_7 _result_7) (`self.Operations`))
                      (bind (_state_8 _optionindex_8) (`self.AddDialog` "Evaluador" (`KismetTextLibrary.Conv_StringToText` _question_7) (`|MakeArray` (`KismetTextLibrary.Conv_IntToText` (`KismetMathLibrary.RandomIntegerInRange` 10 9999)) (`KismetTextLibrary.Conv_IntToText` (`KismetMathLibrary.RandomIntegerInRange` 10 9999)) (`KismetTextLibrary.Conv_IntToText` _result_7))))
                      (switch `/Game/assets/blueprints/enums/Enum_dialog` _state_8
                        (:`NewEnumerator0`
                          (switch `int` _optionindex_8
                            (:`0`
                              _)
                            (:`1`
                              _)
                            (:`2`
                              (set `local.CorrectAmount` (+ (`local.CorrectAmount`) 1))))))))
                  (switch `int` (`self.condition_1`)
                    (:`0`
                      (bind (_question_8 _result_8) (`self.Operations`))
                      (bind (_state_9 _optionindex_9) (`self.AddDialog` "Evaluador" (`KismetTextLibrary.Conv_StringToText` _question_8) (`|MakeArray` (`KismetTextLibrary.Conv_IntToText` _result_8) (`KismetTextLibrary.Conv_IntToText` (`KismetMathLibrary.RandomIntegerInRange` 10 9999)) (`KismetTextLibrary.Conv_IntToText` (`KismetMathLibrary.RandomIntegerInRange` 10 9999)))))
                      (switch `/Game/assets/blueprints/enums/Enum_dialog` _state_9
                        (:`NewEnumerator0`
                          (switch `int` _optionindex_9
                            (:`0`
                              (set `local.CorrectAmount` (+ (`local.CorrectAmount`) 1)))
                            (:`1`
                              _)
                            (:`2`
                              _)))))
                    (:`1`
                      (bind (_question_9 _result_9) (`self.Operations`))
                      (bind (_state_10 _optionindex_10) (`self.AddDialog` "Evaluador" (`KismetTextLibrary.Conv_StringToText` _question_9) (`|MakeArray` (`KismetTextLibrary.Conv_IntToText` (`KismetMathLibrary.RandomIntegerInRange` 10 9999)) (`KismetTextLibrary.Conv_IntToText` _result_9) (`KismetTextLibrary.Conv_IntToText` (`KismetMathLibrary.RandomIntegerInRange` 10 9999)))))
                      (switch `/Game/assets/blueprints/enums/Enum_dialog` _state_10
                        (:`NewEnumerator0`
                          (switch `int` _optionindex_10
                            (:`0`
                              _)
                            (:`1`
                              (set `local.CorrectAmount` (+ (`local.CorrectAmount`) 1)))
                            (:`2`
                              _)))))
                    (:`2`
                      (bind (_question_10 _result_10) (`self.Operations`))
                      (bind (_state_11 _optionindex_11) (`self.AddDialog` "Evaluador" (`KismetTextLibrary.Conv_StringToText` _question_10) (`|MakeArray` (`KismetTextLibrary.Conv_IntToText` (`KismetMathLibrary.RandomIntegerInRange` 10 9999)) (`KismetTextLibrary.Conv_IntToText` (`KismetMathLibrary.RandomIntegerInRange` 10 9999)) (`KismetTextLibrary.Conv_IntToText` _result_10))))
                      (switch `/Game/assets/blueprints/enums/Enum_dialog` _state_11
                        (:`NewEnumerator0`
                          (switch `int` _optionindex_11
                            (:`0`
                              _)
                            (:`1`
                              _)
                            (:`2`
                              (set `local.CorrectAmount` (+ (`local.CorrectAmount`) 1))))))))
                  (switch `int` (`self.condition_2`)
                    (:`0`
                      (bind (_question_11 _result_11) (`self.Operations`))
                      (bind (_state_12 _optionindex_12) (`self.AddDialog` "Evaluador" (`KismetTextLibrary.Conv_StringToText` _question_11) (`|MakeArray` (`KismetTextLibrary.Conv_IntToText` _result_11) (`KismetTextLibrary.Conv_IntToText` (`KismetMathLibrary.RandomIntegerInRange` 10 9999)) (`KismetTextLibrary.Conv_IntToText` (`KismetMathLibrary.RandomIntegerInRange` 10 9999)))))
                      (switch `/Game/assets/blueprints/enums/Enum_dialog` _state_12
                        (:`NewEnumerator0`
                          (switch `int` _optionindex_12
                            (:`0`
                              (set `local.CorrectAmount` (+ (`local.CorrectAmount`) 1)))
                            (:`1`
                              _)
                            (:`2`
                              _)))))
                    (:`1`
                      (bind (_question_12 _result_12) (`self.Operations`))
                      (bind (_state_13 _optionindex_13) (`self.AddDialog` "Evaluador" (`KismetTextLibrary.Conv_StringToText` _question_12) (`|MakeArray` (`KismetTextLibrary.Conv_IntToText` (`KismetMathLibrary.RandomIntegerInRange` 10 9999)) (`KismetTextLibrary.Conv_IntToText` _result_12) (`KismetTextLibrary.Conv_IntToText` (`KismetMathLibrary.RandomIntegerInRange` 10 9999)))))
                      (switch `/Game/assets/blueprints/enums/Enum_dialog` _state_13
                        (:`NewEnumerator0`
                          (switch `int` _optionindex_13
                            (:`0`
                              _)
                            (:`1`
                              (set `local.CorrectAmount` (+ (`local.CorrectAmount`) 1)))
                            (:`2`
                              _)))))
                    (:`2`
                      (bind (_question_13 _result_13) (`self.Operations`))
                      (bind (_state_14 _optionindex_14) (`self.AddDialog` "Evaluador" (`KismetTextLibrary.Conv_StringToText` _question_13) (`|MakeArray` (`KismetTextLibrary.Conv_IntToText` (`KismetMathLibrary.RandomIntegerInRange` 10 9999)) (`KismetTextLibrary.Conv_IntToText` (`KismetMathLibrary.RandomIntegerInRange` 10 9999)) (`KismetTextLibrary.Conv_IntToText` _result_13))))
                      (switch `/Game/assets/blueprints/enums/Enum_dialog` _state_14
                        (:`NewEnumerator0`
                          (switch `int` _optionindex_14
                            (:`0`
                              _)
                            (:`1`
                              _)
                            (:`2`
                              (set `local.CorrectAmount` (+ (`local.CorrectAmount`) 1))))))))
                  (bind _state_15 (`self.AddDialog` "Evaluador" "Perfecto, Evaluemos tus respuestas!" (`|MakeArray` "*Continuar*" :!type "Text")))
                  (switch `/Game/assets/blueprints/enums/Enum_dialog` _state_15
                    (:`NewEnumerator0`
                      (switch `int` 0
                        (:`0`
                          (if (>= (`local.CorrectAmount`) 3)
                            (bind (_state_16 _optionindex_15) (`self.AddDialog` "Evaluador" "APROBASTE! FELICITACIONES!" (`|MakeArray` "VAMOOOOOO!" :!type "Text")))
                            (switch `/Game/assets/blueprints/enums/Enum_dialog` _state_16
                              (:`NewEnumerator0`
                                (switch `int` _optionindex_15
                                  (:`0`
                                    (`self.ClearDialogProgress`)
                                    (`self.CloseDialog`)
                                    (`/Engine/EditorBlueprintResources/StandardMacros.DoOnce` false
                                      (:`Completed`
                                        (cast `/Game/assets/blueprints/Camara` (`GameplayStatics.GetGameMode`))
                                        (`GameplayStatics.OpenLevel` "MAP_2d_4")))))))
                            (else
                              (bind (_state_17 _optionindex_16) (`self.AddDialog` "Evaluador" "Lamento decirtelo, pero no aprobaste. intentalo de nuevo mas tarde" (`|MakeArray` "Oh...." :!type "Text")))
                              (switch `/Game/assets/blueprints/enums/Enum_dialog` _state_17
                                (:`NewEnumerator0`
                                  (switch `int` _optionindex_16
                                    (:`0`
                                      (`self.SetDialogTreeIndex` 1)
                                      (`self.CloseDialog`))))))))))))))
            (:`1`
              (bind (_state_18 _optionindex_17) (`self.AddDialog` "Evaluador" "Bueno, esta bien, tomate tu tiempo" (`|MakeArray` "*Continuar*" :!type "Text")))
              (switch `/Game/assets/blueprints/enums/Enum_dialog` _state_18
                (:`NewEnumerator0`
                  (switch `int` _optionindex_17
                    (:`0`
                      (`self.SetDialogTreeIndex` 1)
                      (`self.CloseDialog`))))))))))
    (:`1`
      (bind (_state_19 _optionindex_18) (`self.AddDialog` "Evaluador" "Lista?" (`|MakeArray` "Si" "No" :!type "Text")))
      (switch `/Game/assets/blueprints/enums/Enum_dialog` _state_19
        (:`NewEnumerator0`
          (switch `int` _optionindex_18
            (:`0`
              (goto _label))
            (:`1`
              (`self.ClearDialogProgress`)
              (`self.CloseDialog`))))))))

(fn `Operations`
  (returns (Question :type String) (Result :type Integer))
  (bind _num_a (`self.num A`))
  (bind _num_b_ (`self.num B `))
  (bind _num_a_2 (`self.num A`))
  (bind _num_b__2 (`self.num B `))
  (bind _returnvalue (`KismetStringLibrary.Conv_IntToString` _num_a_2))
  (bind _returnvalue_2 (`KismetStringLibrary.Conv_IntToString` _num_b__2))
  (set `self.num A` (`KismetMathLibrary.RandomIntegerInRange` 10 99))
  (set `self.num B ` (`KismetMathLibrary.RandomIntegerInRange` 10 99))
  (if (== _num_a (* (/ _num_a _num_b_) _num_b_))
    (set `self.div_or_not` 1)
    (else
      (set `self.div_or_not` 1)))
  (switch `int` (`KismetMathLibrary.RandomIntegerInRange` 0 (`self.div_or_not`))
    (:`0`
      (return (`KismetStringLibrary.Concat_StrStr` _returnvalue "+" _returnvalue_2 "?") (+ _num_a_2 _num_b__2)))
    (:`1`
      (return (`KismetStringLibrary.Concat_StrStr` _returnvalue "-" _returnvalue_2 "?") (- _num_a_2 _num_b__2)))
    (:`2`
      (return (`KismetStringLibrary.Concat_StrStr` _returnvalue "*" _returnvalue_2 "?") (* _num_a_2 _num_b__2)))
    (:`3`
      (return (`KismetStringLibrary.Concat_StrStr` _returnvalue "/" _returnvalue_2 "?") (/ _num_a_2 _num_b__2)))))