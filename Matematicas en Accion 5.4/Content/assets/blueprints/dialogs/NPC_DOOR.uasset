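; NPC_DOOR is an interactable dialog actor, likely a door, that starts a conversation when a player interacts with it.
; Interact stores the instigator, starts the ACDialogDOOR dialog component at index 0, and prints the Hola flag for debugging.
; A separate Destruct function destroys the actor when Hola is true; nothing in this Blueprint calls it or sets that flag.
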(event `self.Interact`
  (params (instigator :type "Actor Object Reference"))
  (set `self.InteractInstigator` instigator)
  (`/Game/assets/blueprints/dialogs/AC_DialogBase.StartDialog` (`self.AC_Dialog_DOOR`) 0)
  (`KismetSystemLibrary.PrintString` (`KismetStringLibrary.Conv_BoolToString` (`self.hola`))))

(fn `destruct`
  (if (`self.hola`)
    (`self.K2_DestroyActor`)))

(fn `UserConstructionScript`
  (`parent.UserConstructionScript`))