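; Door dialog component where a mysterious speaker poses a random arithmetic question as the condition to pass.
; Dialog randomly places the result from Operations among three options, with random numbers as decoys.
; A correct answer clears dialog progress and closes, while a wrong one switches to a returning-visitor greeting that can retry.
; The MakeQuestion flag guards question generation until an answer resets it.
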(fn `Dialog`
  (locals (CorrectAmount :type Integer))
  (bind _returnvalue (`KismetMathLibrary.RandomIntegerInRange` 0 2))
  (`parent.Dialog`)
  (switch `int` (`self.DialogTreeIndex`)
    (:`0`
      (bind (_state _optionindex) (`self.AddDialog` "¿?" "Responde a mi pregunta para pasar...." (`|MakeArray` "*CONTINUAR*" :!type "Text")))
      (switch `/Game/assets/blueprints/enums/Enum_dialog` _state
        (:`NewEnumerator0`
          (switch `int` _optionindex
            (:`0`
              (if (not (`self.MakeQuestion`)) :!label _label
                (`KismetSystemLibrary.PrintString` (`KismetStringLibrary.Conv_IntToString` _returnvalue))
                (set `self.MakeQuestion` true)
                (switch `int` _returnvalue
                  (:`0`
                    (bind (_question _result) (`self.Operations`))
                    (`KismetSystemLibrary.PrintString` (`KismetStringLibrary.Conv_IntToString` _result))
                    (bind (_state_2 _optionindex_2) (`self.AddDialog` "Evaluador" (`KismetTextLibrary.Conv_StringToText` _question) (`|MakeArray` (`KismetTextLibrary.Conv_IntToText` _result) (`KismetTextLibrary.Conv_IntToText` (`KismetMathLibrary.RandomIntegerInRange` 1 99)) (`KismetTextLibrary.Conv_IntToText` (`KismetMathLibrary.RandomIntegerInRange` 1 99)))))
                    (switch `/Game/assets/blueprints/enums/Enum_dialog` _state_2
                      (:`NewEnumerator0`
                        (switch `int` _optionindex_2
                          (:`0`
                            (bind (_state_3 _optionindex_3) (`self.AddDialog` "¿?" "Respuesta....CORRECTA!" (`|MakeArray` "*CONTINUAR*" :!type "Text") :!label _label_2))
                            (switch `/Game/assets/blueprints/enums/Enum_dialog` _state_3
                              (:`NewEnumerator0`
                                (switch `int` _optionindex_3
                                  (:`0`
                                    (set `self.MakeQuestion` false)
                                    (`self.ClearDialogProgress`)
                                    (`self.CloseDialog`))))))
                          (:`1`
                            (bind (_state_4 _optionindex_4) (`self.AddDialog` "Evaluador" "Respuesta... INCORRECTA!!!" (`|MakeArray` "Oh...." :!type "Text") :!label _label_3))
                            (switch `/Game/assets/blueprints/enums/Enum_dialog` _state_4
                              (:`NewEnumerator0`
                                (switch `int` _optionindex_4
                                  (:`0`
                                    (set `self.MakeQuestion` false)
                                    (`self.SetDialogTreeIndex` 1)
                                    (`self.CloseDialog`))))))
                          (:`2`
                            (goto _label_3))))))
                  (:`1`
                    (bind (_question_2 _result_2) (`self.Operations`))
                    (`KismetSystemLibrary.PrintString` (`KismetStringLibrary.Conv_IntToString` _result_2))
                    (bind (_state_5 _optionindex_5) (`self.AddDialog` "Evaluador" (`KismetTextLibrary.Conv_StringToText` _question_2) (`|MakeArray` (`KismetTextLibrary.Conv_IntToText` (`KismetMathLibrary.RandomIntegerInRange` 1 99)) (`KismetTextLibrary.Conv_IntToText` _result_2) (`KismetTextLibrary.Conv_IntToText` (`KismetMathLibrary.RandomIntegerInRange` 1 99)))))
                    (switch `/Game/assets/blueprints/enums/Enum_dialog` _state_5
                      (:`NewEnumerator0`
                        (switch `int` _optionindex_5
                          (:`0`
                            (goto _label_3))
                          (:`1`
                            (goto _label_2))
                          (:`2`
                            (goto _label_3))))))
                  (:`2`
                    (bind (_question_3 _result_3) (`self.Operations`))
                    (`KismetSystemLibrary.PrintString` (`KismetStringLibrary.Conv_IntToString` _result_3))
                    (bind (_state_6 _optionindex_6) (`self.AddDialog` "Evaluador" (`KismetTextLibrary.Conv_StringToText` _question_3) (`|MakeArray` (`KismetTextLibrary.Conv_IntToText` (`KismetMathLibrary.RandomIntegerInRange` 1 99)) (`KismetTextLibrary.Conv_IntToText` (`KismetMathLibrary.RandomIntegerInRange` 1 99)) (`KismetTextLibrary.Conv_IntToText` _result_3))))
                    (switch `/Game/assets/blueprints/enums/Enum_dialog` _state_6
                      (:`NewEnumerator0`
                        (switch `int` _optionindex_6
                          (:`0`
                            (goto _label_3))
                          (:`1`
                            (goto _label_3))
                          (:`2`
                            (goto _label_2)))))))))))))
    (:`1`
      (bind (_state_7 _optionindex_7) (`self.AddDialog` "¿?" "Vienes otra vez...??" (`|MakeArray` "*CONTINUAR*" :!type "Text")))
      (switch `/Game/assets/blueprints/enums/Enum_dialog` _state_7
        (:`NewEnumerator0`
          (switch `int` _optionindex_7
            (:`0`
              (goto _label))
            (:`1`
              (`self.ClearDialogProgress`)
              (`self.CloseDialog`))))))))

(fn `Operations`
  (returns (Question :type String) (Result :type Integer))
  (bind _returnvalue (`KismetMathLibrary.RandomIntegerInRange` 1 9))
  (bind _returnvalue_2 (`KismetMathLibrary.RandomIntegerInRange` 1 9))
  (bind _returnvalue_3 (`KismetStringLibrary.Conv_IntToString` _returnvalue_2))
  (bind _returnvalue_4 (`KismetStringLibrary.Conv_IntToString` _returnvalue))
  (switch `int` (`KismetMathLibrary.RandomIntegerInRange` 0 3)
    (:`0`
      (return (`KismetStringLibrary.Concat_StrStr` _returnvalue_3 "+" _returnvalue_4 "?") (+ _returnvalue_2 _returnvalue)))
    (:`1`
      (return (`KismetStringLibrary.Concat_StrStr` _returnvalue_3 "-" _returnvalue_4 "?") (- _returnvalue_2 _returnvalue)))
    (:`2`
      (return (`KismetStringLibrary.Concat_StrStr` _returnvalue_3 "*" _returnvalue_4 "?") (* _returnvalue_2 _returnvalue)))
    (:`3`
      (return (`KismetStringLibrary.Concat_StrStr` _returnvalue_3 "/" _returnvalue_4 "?") (/ _returnvalue_2 _returnvalue)))))