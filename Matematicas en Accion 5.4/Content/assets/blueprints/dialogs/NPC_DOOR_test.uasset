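; Test Blueprint for a door NPC that opens a randomly chosen dialog when interacted with.
; Interact stores the instigator, passes a random 0 or 1 to StartDialog on the ACDialogDOORTest component, then prints the Hola flag for debugging.
; A separate Destruct function destroys the actor when Hola is true, though nothing in this graph calls it or sets that flag.
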(event `self.Interact`
  (params (instigator :type "Actor Object Reference"))
  (set `self.NewVar` (`KismetMathLibrary.RandomIntegerInRange` 0 1))
  (set `self.InteractInstigator` instigator)
  (`/Game/assets/blueprints/dialogs/AC_DialogBase.StartDialog` (`self.AC_Dialog_DOOR_Test`) (`self.NewVar`))
  (`KismetSystemLibrary.PrintString` (`KismetStringLibrary.Conv_BoolToString` (`self.hola`))))

(fn `destruct`
  (if (`self.hola`)
    (`self.K2_DestroyActor`)))

(fn `UserConstructionScript`
  (`parent.UserConstructionScript`))