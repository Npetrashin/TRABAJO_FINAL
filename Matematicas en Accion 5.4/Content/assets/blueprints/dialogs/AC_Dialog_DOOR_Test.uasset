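; Test dialog component for a door that poses a random arithmetic question as a multiple-choice gate, with Spanish text.
; Operations builds the question and result from separate random rolls, so they can disagree.
; Condition places that result first or second among random decoys; picking it clears progress and closes the dialog, others show "incorrecto".
; A repeat-visit branch exists, but the failure path that would select it is unconnected.
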(fn `Dialog`
  (locals (CorrectAmount :type Integer))
  (`parent.Dialog`)
  (`KismetSystemLibrary.PrintString` (`KismetStringLibrary.Conv_IntToString` (`self.condition`)))
  (switch `int` (`self.DialogTreeIndex`)
    (:`0`
      (bind (_state _optionindex) (`self.AddDialog` "¿?" "Responde a mi pregunta para pasar...." (`|MakeArray` "*CONTINUAR*" :!type "Text")))
      (switch `/Game/assets/blueprints/enums/Enum_dialog` _state
        (:`NewEnumerator0`
          (switch `int` _optionindex
            (:`0`
              (bind (_question _result) (`self.Operations`))
              (switch `int` (`self.condition`)
                (:`0`
                  (bind (_state_2 _optionindex_2) (`self.AddDialog` "¿?" (`KismetTextLibrary.Conv_StringToText` _question) (`|MakeArray` (`KismetTextLibrary.Conv_IntToText` _result) (`KismetTextLibrary.Conv_IntToText` (`KismetMathLibrary.RandomIntegerInRange` 1 99)) (`KismetTextLibrary.Conv_IntToText` (`KismetMathLibrary.RandomIntegerInRange` 1 99)))))
                  (switch `/Game/assets/blueprints/enums/Enum_dialog` _state_2
                    (:`NewEnumerator0`
                      (switch `int` _optionindex_2
                        (:`0`
                          (bind (_state_3 _optionindex_3) (`self.AddDialog` "¿?" "Respuesta....CORRECTA!" (`|MakeArray` "*CONTINUAR*" :!type "Text") :!label _label))
                          (switch `/Game/assets/blueprints/enums/Enum_dialog` _state_3
                            (:`NewEnumerator0`
                              (switch `int` _optionindex_3
                                (:`0`
                                  (`self.ClearDialogProgress`)
                                  (`self.CloseDialog`))))))
                        (:`1`
                          (`self.AddDialog` "¿?" "incorrecto" :!label _label_2))
                        (:`2`
                          (goto _label_2))))))
                (:`1`
                  (bind (_state_4 _optionindex_4) (`self.AddDialog` "¿?" (`KismetTextLibrary.Conv_StringToText` _question) (`|MakeArray` (`KismetTextLibrary.Conv_IntToText` (`KismetMathLibrary.RandomIntegerInRange` 1 99)) (`KismetTextLibrary.Conv_IntToText` _result) (`KismetTextLibrary.Conv_IntToText` (`KismetMathLibrary.RandomIntegerInRange` 1 99)))))
                  (switch `/Game/assets/blueprints/enums/Enum_dialog` _state_4
                    (:`NewEnumerator0`
                      (switch `int` _optionindex_4
                        (:`0`
                          (goto _label_2))
                        (:`1`
                          (goto _label))
                        (:`2`
                          (goto _label_2))))))))))))
    (:`1`
      (bind (_state_5 _optionindex_5) (`self.AddDialog` "¿?" "Vienes otra vez...??" (`|MakeArray` "*CONTINUAR*" :!type "Text")))
      (switch `/Game/assets/blueprints/enums/Enum_dialog` _state_5
        (:`NewEnumerator0`
          (switch `int` _optionindex_5
            (:`1`
              (`self.ClearDialogProgress`)
              (`self.CloseDialog`))))))))

(fn `Operations`
  (returns (Question :type String) (Result :type Integer))
  (bind _returnvalue (`KismetMathLibrary.RandomIntegerInRange` 1 9))
  (bind _returnvalue_2 (`KismetMathLibrary.RandomIntegerInRange` 1 9))
  (bind _returnvalue_3 (`KismetStringLibrary.Conv_IntToString` _returnvalue_2))
  (bind _returnvalue_4 (`KismetStringLibrary.Conv_IntToString` _returnvalue))
  (switch `int` (`KismetMathLibrary.RandomIntegerInRange` 0 3)
    (:`0`
      (return (`KismetStringLibrary.Concat_StrStr` _returnvalue_3 "+" _returnvalue_4 "?") (+ _returnvalue_2 _returnvalue)))
    (:`1`
      (return (`KismetStringLibrary.Concat_StrStr` _returnvalue_3 "-" _returnvalue_4 "?") (- _returnvalue_2 _returnvalue)))
    (:`2`
      (return (`KismetStringLibrary.Concat_StrStr` _returnvalue_3 "*" _returnvalue_4 "?") (* _returnvalue_2 _returnvalue)))
    (:`3`
      (return (`KismetStringLibrary.Concat_StrStr` _returnvalue_3 "/" _returnvalue_4 "?") (/ _returnvalue_2 _returnvalue)))))