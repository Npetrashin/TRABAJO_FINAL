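; Base Blueprint for dialog NPCs that show a floating character name and take part in conversations.
; The construction script fills the name text component from CharacterName.
; SetInteractableState toggles that text's visibility according to whether interaction is available.
; ConversationClosed notifies the stored InteractInstigator through its ConversationClosedMessage.
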(event `/Game/assets/blueprints/dialogs/BPI_Interactable.SetInteractableState`
  (params (CanShowInteract :type Boolean))
  (if CanShowInteract
    (`SceneComponent.SetVisibility` (`self.TXT_CharName`) true false)
    (else
      (`SceneComponent.SetVisibility` (`self.TXT_CharName`) false false))))

(event `/Game/assets/blueprints/dialogs/BPI_Interactable.ConversationClosed`
  (message `/Game/assets/blueprints/dialogs/BPI_Interactable.ConversationClosed` (`self.InteractInstigator`)))

(fn `UserConstructionScript`
  (`TextRenderComponent.K2_SetText` (`self.TXT_CharName`) (`self.CharacterName`)))