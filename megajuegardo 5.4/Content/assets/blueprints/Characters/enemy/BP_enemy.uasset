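; BP_enemy is an enemy character that targets the player on proximity and drops currency when defeated.
; When a BP_Player begins overlapping its AggroRange component, it passes that player to its AIC_Enemy controller through GetAttackTarget.
; On BeginPlay it binds OnDeath to the Defeated event, which spawns a Currency_BP at the enemy's location and rotation.
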(event `self.ReceiveBeginPlay`
  (`parent.ReceiveBeginPlay`)
  (add `self.Defeated` (delegate `OnDeath`)))

(event `OnDeath`
  (bind (_returnvalue_location _returnvalue_rotation) (`KismetMathLibrary.BreakTransform` (`self.GetTransform`)))
  (`|SpawnActorFromClass` "/Game/assets/blueprints/Abilities/currency_BP.currency_BP_C" (`KismetMathLibrary.MakeTransform` _returnvalue_location _returnvalue_rotation) "Undefined" "MultiplyWithRoot" null null))

(event `self.AggroRange.OnComponentBeginOverlap`
  (params (OverlappedComponent :type "PrimitiveComponent Object Reference") (OtherActor :type "Actor Object Reference") (OtherComp :type "PrimitiveComponent Object Reference") (OtherBodyIndex :type Integer) (bFromSweep :type Boolean) (SweepResult :type "HitResult Structure (by ref)"))
  (bind _asbp_player (cast `/Game/assets/blueprints/Characters/chie/BP_Player` OtherActor))
  (bind _asaic_enemy (cast `/Game/assets/blueprints/AI/AIC_Enemy` (`AIBlueprintHelperLibrary.GetAIController` self)))
  (`/Game/assets/blueprints/AI/AIC_Enemy.Get Attack Target` _asaic_enemy _asbp_player))

(fn `UserConstructionScript`
  (`parent.UserConstructionScript`))