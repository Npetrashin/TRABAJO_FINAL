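; Player character for a 2D platformer, with Enhanced Input movement, jumping, attacks, pausing and a money HUD.
; Actions are gated by CanAct; attacks play animation overrides that set IsAttacking, and the unlockable throw replaces any active BP_Ruler projectile.
; An overlap range tracks one BPI_Interactable for UI-mode conversations.
; It also keeps a Notes counter, grants abilities like double jump, and restarts the game after death.
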(event `self.ReceiveBeginPlay`
  (`parent.ReceiveBeginPlay`)
  (bind _asplayer_controller (cast `PlayerController` (`self.GetController`)))
  (`EnhancedInputSubsystemInterface.AddMappingContext` (pcsubsystem `EnhancedInputLocalPlayerSubsystem` _asplayer_controller) "/Game/input/plataformeo_mov.plataformeo_mov" 0 (struct))
  (bind _returnvalue (`|CreateWidget` "/Game/UI/Current_money.Current_money_C"))
  (`UserWidget.AddToViewport` _returnvalue 0)
  (add `self.Defeated` (delegate `OnDeath`)))

(event `OnDeath`
  (`SceneComponent.K2_SetRelativeLocation` (`self.Sprite`) (`SceneComponent.RelativeLocation` (`self.fix`)) false false)
  (bind _ascamara (cast `/Game/assets/blueprints/Camara` (`GameplayStatics.GetGameMode`)))
  (`KismetSystemLibrary.Delay` 1.0)
  (`/Game/assets/blueprints/Camara.RestartGame` _ascamara))

(event `EnhancedInput|/Game/input/acciones/salto`
  (params (ActionValue :type Boolean) (ElapsedSeconds :type "Float (double-precision)") (TriggeredSeconds :type "Float (double-precision)") (InputAction :type "InputAction Object Reference" :default "/Game/input/acciones/salto.salto"))
  (:`Started`
    (if (`self.CanAct`)
      (`self.Jump`)))
  (:`Completed`
    (`self.StopJumping`)))

(event `EnhancedInput|/Game/input/acciones/moverse`
  (params (ActionValue :type "Float (double-precision)") (ElapsedSeconds :type "Float (double-precision)") (TriggeredSeconds :type "Float (double-precision)") (InputAction :type "InputAction Object Reference" :default "/Game/input/acciones/moverse.moverse"))
  (:`Triggered`
    (if (`self.CanAct`)
      (`self.AddMovementInput` (1.0 0.0 0.0) (`KismetMathLibrary.BreakVector2D` (`KismetMathLibrary.Conv_DoubleToVector2D` ActionValue)))
      (`Controller.SetControlRotation` (`self.GetController`) (select `bool` (> ActionValue 0.0) :`false` (`KismetMathLibrary.MakeRotator` 0.0 0.0 180.0) :`true` (`KismetMathLibrary.MakeRotator` 0.0))))))

(event `EnhancedInput|/Game/input/acciones/PAUSA`
  (params (ActionValue :type Boolean) (ElapsedSeconds :type "Float (double-precision)") (TriggeredSeconds :type "Float (double-precision)") (InputAction :type "InputAction Object Reference" :default "/Game/input/acciones/PAUSA.PAUSA"))
  (bind _returnvalue (`GameplayStatics.GetPlayerController` 0))
  (:`Started`
    (bind _returnvalue_2 (`|CreateWidget` "/Game/UI/pausa.pausa_C"))
    (`UserWidget.AddToViewport` _returnvalue_2 0)
    (set `PlayerController.bShowMouseCursor` true _returnvalue)
    (`WidgetBlueprintLibrary.SetInputMode_UIOnlyEx` _returnvalue null)
    (`GameplayStatics.SetGamePaused` true)))

(event `EnhancedInput|/Game/input/acciones/Ataque`
  (params (ActionValue :type Boolean) (ElapsedSeconds :type "Float (double-precision)") (TriggeredSeconds :type "Float (double-precision)") (InputAction :type "InputAction Object Reference" :default "/Game/input/acciones/Ataque.Ataque"))
  (:`Started`
    (if (`self.CanAct`)
      (`PaperZDPlaySlotOverrideAction.PlayAnimationOverrideWithCallbacks` (`self.GetAnimInstance`) "/Game/assets/blueprints/AnimSequences/attack1.attack1" "ataque"
        (:`then`
          (set `self.IsAttacking` true))
        (:`OnCompleted`
          (set `self.IsAttacking` false :!label _label))
        (:`OnCancelled`
          (goto _label))))))

(event `EnhancedInput|/Game/input/acciones/Lanzamiento`
  (params (ActionValue :type Boolean) (ElapsedSeconds :type "Float (double-precision)") (TriggeredSeconds :type "Float (double-precision)") (InputAction :type "InputAction Object Reference" :default "/Game/input/acciones/Lanzamiento.Lanzamiento"))
  (bind (_returnvalue_location _returnvalue_rotation) (`KismetMathLibrary.BreakTransform` (`self.GetTransform`)))
  (:`Started`
    (if (`self.CanAct`)
      (if (`KismetArrayLibrary.Array_Contains` (`self.Unlocked_Abilities`) "NewEnumerator1")
        (`|ExecutionSequence`
          (:`then_0`
            (`/Engine/EditorBlueprintResources/StandardMacros.IsValid` (`self.Active Sword`)
              (:`Is Valid`
                (`self.K2_DestroyActor` (`self.Active Sword`)))))
          (:`then_1`
            (`PaperZDPlaySlotOverrideAction.PlayAnimationOverrideWithCallbacks` (`self.GetAnimInstance`) "/Game/assets/blueprints/Characters/chie/AnimSequences/Throw.Throw" "ataque"
              (:`then`
                (bind _returnvalue (`|SpawnActorFromClass` "/Game/assets/blueprints/Abilities/BP_Ruler.BP_Ruler_C" (`KismetMathLibrary.MakeTransform` _returnvalue_location _returnvalue_rotation) "AlwaysSpawn" "MultiplyWithRoot" null null))
                (set `self.Active Sword` _returnvalue)
                (set `self.IsAttacking` true))
              (:`OnCompleted`
                (set `self.IsAttacking` false :!label _label_2))
              (:`OnCancelled`
                (goto _label_2)))))))))

(event `EnhancedInput|/Game/input/acciones/Interact`
  (params (ActionValue :type Boolean) (ElapsedSeconds :type "Float (double-precision)") (TriggeredSeconds :type "Float (double-precision)") (InputAction :type "InputAction Object Reference" :default "/Game/input/acciones/Interact.Interact"))
  (bind _returnvalue (`GameplayStatics.GetPlayerController` 0))
  (:`Started`
    (`/Engine/EditorBlueprintResources/StandardMacros.IsValid` (`self.Interactable`)
      (:`Is Valid`
        (message `/Game/assets/blueprints/dialogs/BPI_Interactable.Interact` (`self.Interactable`) self)
        (`WidgetBlueprintLibrary.SetInputMode_UIOnlyEx` _returnvalue null)
        (set `PlayerController.bShowMouseCursor` true _returnvalue)))))

(event `self.InteractRange.OnComponentBeginOverlap`
  (params (OverlappedComponent :type "PrimitiveComponent Object Reference") (OtherActor :type "Actor Object Reference") (OtherComp :type "PrimitiveComponent Object Reference") (OtherBodyIndex :type Integer) (bFromSweep :type Boolean) (SweepResult :type "HitResult Structure (by ref)"))
  (if (!= OtherActor self)
    (if (`KismetSystemLibrary.DoesImplementInterface` OtherActor "/Game/assets/blueprints/dialogs/BPI_Interactable.BPI_Interactable_C")
      (`/Engine/EditorBlueprintResources/StandardMacros.IsValid` (`self.Interactable`)
        (:`Is Valid`
          (message `/Game/assets/blueprints/dialogs/BPI_Interactable.SetInteractableState` (`self.Interactable`) false)
          (set `self.Interactable` null))
        (:`Is Not Valid`
          _))
      (set `self.Interactable` OtherActor)
      (message `/Game/assets/blueprints/dialogs/BPI_Interactable.SetInteractableState` (`self.Interactable`) true))))

(event `self.InteractRange.OnComponentEndOverlap`
  (params (OverlappedComponent :type "PrimitiveComponent Object Reference") (OtherActor :type "Actor Object Reference") (OtherComp :type "PrimitiveComponent Object Reference") (OtherBodyIndex :type Integer))
  (if (and (!= OtherActor self) (== (`self.Interactable`) OtherActor))
    (message `/Game/assets/blueprints/dialogs/BPI_Interactable.SetInteractableState` (`self.Interactable`) false)
    (set `self.Interactable` null)))

(event `/Game/assets/blueprints/dialogs/BPI_Interactable.ConversationClosed`
  (bind _returnvalue (`GameplayStatics.GetPlayerController` 0))
  (set `PlayerController.bShowMouseCursor` false _returnvalue)
  (`WidgetBlueprintLibrary.SetInputMode_GameOnly` _returnvalue))

(event `add notes`
  (params (`Added notes` :type Integer))
  (set `self.Notes` (+ `Added notes` (`self.Notes`))))

(event `remove notes`
  (params (B :type Integer))
  (set `self.Notes` (- (`self.Notes`) B)))

(fn `GainAbility`
  (params (AbilityType :type "/Game/assets/blueprints/enums/E_Abilities Enum (by ref)"))
  (`KismetArrayLibrary.Array_AddUnique` (`self.Unlocked_Abilities`) AbilityType)
  (switch `/Game/assets/blueprints/enums/E_Abilities` (`local.AbilityType`)
    (:`NewEnumerator0`
      (set `self.JumpMaxCount` 2))))

(fn `UserConstructionScript`
  (`parent.UserConstructionScript`))