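; BP_ActionChar is an action-combat character with health, factions, a toggleable melee hitbox and stun and defeat states.
; Hitbox overlaps with another faction's BP_ActionChar deal fixed damage and briefly freeze both characters through CustomTimeDilation for hit stop.
; ReceiveAttack jumps the animation state machine to stun or death, fires the matching dispatcher, and starts a stun timer or disables capsule collision.
; CanAct gates actions on attacking, stunned and defeated flags.
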(event `self.ReceiveBeginPlay`
  (`self.set hitbox collission` false)
  (set `self.Current Health` (`self.Max Health`)))

(event `self.hitbox.OnComponentBeginOverlap`
  (params (OverlappedComponent :type "PrimitiveComponent Object Reference") (OtherActor :type "Actor Object Reference") (OtherComp :type "PrimitiveComponent Object Reference") (OtherBodyIndex :type Integer) (bFromSweep :type Boolean) (SweepResult :type "HitResult Structure (by ref)"))
  (bind _asbp_action_char (cast `/Game/assets/blueprints/Characters/BP_ActionChar` OtherActor))
  (if (!= (`/Game/assets/blueprints/Characters/BP_ActionChar.faction` _asbp_action_char) (`self.faction`))
    (`self.receive attack` _asbp_action_char 25.0)
    (`self.HitStop Sequence` _asbp_action_char 0.2)
    (`self.HitStop Sequence` 0.2)))

(event `HitStop Sequence`
  (params (Duration :type "Float (single-precision)" :default 0.2))
  (set `self.CustomTimeDilation` 0.0)
  (`KismetSystemLibrary.RetriggerableDelay` Duration)
  (set `self.CustomTimeDilation` 1.0))

(fn `CanAct`
  (returns (CanAct :type Boolean))
  (return (and (not (`self.IsAttacking`)) (not (`self.IsDefeated`)) (not (`self.IsStunned`)))))

(fn `clear stun`
  (bind _output_get (set `self.IsStunned` false))
  (`self.StunStateChange` _output_get))

(fn `receive attack`
  (params (Damage :type "Float (double-precision)" :default 25.0))
  (if (not (`self.IsDefeated`))
    (set `self.Current Health` (- (`self.Current Health`) (`local.Damage`)))
    (`PaperZDAnimInstance.StopAllAnimationOverrides` (`self.GetAnimInstance`))
    (if (<= (`self.Current Health`) 0.0)
      (`PaperZDAnimInstance.JumpToNode` (`self.GetAnimInstance`) "Jump_Ded" "None")
      (set `self.IsDefeated` true)
      (`PrimitiveComponent.SetCollisionEnabled` (`self.CapsuleComponent`) "NoCollision")
      (`self.Defeated`)
      (else
        (bind _output_get (set `self.IsStunned` true))
        (`self.StunStateChange` _output_get)
        (`PaperZDAnimInstance.JumpToNode` (`self.GetAnimInstance`) "Jump_stun" "None")
        (`KismetSystemLibrary.K2_SetTimerDelegate` (`|CreateDelegate` :!event `clear stun`) (`self.StunLenght`))))))

(fn `set hitbox collission`
  (params (IsActive :type Boolean))
  (if IsActive
    (`PrimitiveComponent.SetCollisionEnabled` (`self.hitbox`) "QueryOnly")
    (else
      (`PrimitiveComponent.SetCollisionEnabled` (`self.hitbox`) "NoCollision"))))

(fn `UserConstructionScript`)